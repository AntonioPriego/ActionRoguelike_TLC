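; Projectile cannon actor that fires magic projectiles at regular intervals.
; A looping timer started at BeginPlay spawns MagicProjectileBP at the Arrow component's world location and rotation.
; When FollowsPlayer is set, Tick turns the Arrow toward the player pawn each frame using a look-at rotation from the actor's location, so shots track the player.
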(event Custom|OnTimerElapsed
  (bind _arrow (Variables|Default|GetArrow))
  (Game|SpawnActorfromClass "/Game/MagicProjectileBP.MagicProjectileBP_C" (Math|Transform|MakeTransform (Transformation|GetWorldLocation _arrow) (Transformation|GetWorldRotation _arrow)) "Undefined" 0 0))

(event EventBeginPlay
  (Utilities|Time|SetTimerbyEvent (delegate Custom|OnTimerElapsed) 2.0 true))

(event EventTick
  (params (DeltaSeconds :type Float%20%28single-precision%29))
  (if (Variables|Default|GetFollowsPlayer)
    (Transformation|SetWorldRotation (Variables|Default|GetArrow) (Math|Rotator|FindLookatRotation (Transformation|GetActorLocation) (Transformation|GetActorLocation (Game|Player|GetPlayerPawn 0))) false false)))

(fn ConstructionScript)