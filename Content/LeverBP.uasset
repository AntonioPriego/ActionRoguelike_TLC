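; Interactable lever Blueprint that grants the KeyCard gameplay tag to the pawn that uses it.
; Interact flips the handle mesh pitch up or down through a FlipFlop, then adds the tag to the active tags on the instigator's SActionComponent on every use.
; An unconnected leftover branch would forward interaction to a selected actor or explode an ExplosiveBarrelBP.
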(event EventBeginPlay)

(event Collision|EventActorBeginOverlap
  (params (OtherActor :type Actor%20Object%20Reference)))

(event EventTick
  (params (DeltaSeconds :type Float%20%28single-precision%29)))

(event EventInteract
  (params (InstigatorPawn :type Pawn%20Object%20Reference))
  ;[0.3229 1 0.3287] Lever anim up/down
  (bind _isa (Utilities|FlowControl|FlipFlop)
    (:A
      _)
    (:B
      _))
  (Transformation|SetRelativeRotation (Variables|Default|GetHandleMesh) (select _isa (Math|Rotator|MakeRotator 0.0 -3e+01 0.0) (Math|Rotator|MakeRotator 0.0 3e+01 0.0)) false false)
  ;[0.3229 1 0.3287] Interact action
  (GameplayTags|AddGameplayTag (Variables|/Script/ActionRoguelike_TLC.SActionComponent|GetActiveGameplayTags (Actor|GetComponentbyClass InstigatorPawn "/Script/ActionRoguelike_TLC.SActionComponent")) (Variables|Default|GetKeyCard) :!class /Script/GameplayTags.BlueprintGameplayTagLibrary))

(fn ConstructionScript)