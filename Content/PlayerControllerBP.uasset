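; Player controller that finishes player-state-dependent setup and hosts the pause menu, alongside temporary debug keys.
; On entering the playing state, it notifies the PlayerCharacter that PlayerState is set, so dependent widgets can work.
; Only local controllers create the pause widget, which is added to the viewport collapsed.
; Debug keys trigger a world save through SGameModeBase and set or print the round personal best on SPlayerState.
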(event EventBeginPlay)

(event EventTick
  (params (DeltaSeconds :type Float%20%28single-precision%29)))

(event EventBlueprintBeginPlayingState
  (bind _self self)
  ;[0.3229 1 0.3287] Notify to PlayerCharacter PlayerState is setted to be able to work with some widgets that need it
  (bind _asplayer_character (Utilities|Casting|CastToPlayerCharacter (Game|GetPlayerCharacter 0)))
  (Default|PlayerStateSetted _asplayer_character)
  ;[0.3229 1 0.3287] Create PauseWidget only on local instances
  (if (Pawn|IsLocalController)
    (bind _returnvalue (UserInterface|CreateWidget "/Game/UI/Menu/PauseMenu_Widget.PauseMenu_Widget_C" _self _self))
    (bind _output_get (Variables|Default|SetPauseMenuInstance _returnvalue))
    (UserInterface|Viewport|AddtoViewport _output_get 0)
    (Widget|SetVisibility _output_get "Collapsed")))

(event Input|KeyboardEvents|DebugKeyB
  (params (Key :type Key%20Structure :default "None") (ActionValue :type Input%20Action%20Value%20Structure))
  ;[1 0 0] DEBUG
  (:Pressed
    (bind _assplayer_state (Utilities|Casting|CastToSPlayerState (Variables|Default|GetPlayerState)))
    (Class|SPlayerState|SetRoundPersonalBest _assplayer_state 2)
    (Development|PrintString "2" true true "(R=1.000000,G=0.000000,B=0.365323,A=1.000000)")))

(event Input|KeyboardEvents|DebugKeyN
  (params (Key :type Key%20Structure :default "None") (ActionValue :type Input%20Action%20Value%20Structure))
  ;[1 0 0] DEBUG
  (:Pressed
    (bind _assplayer_state (Utilities|Casting|CastToSPlayerState (Variables|Default|GetPlayerState)))
    (Development|PrintString (Utilities|String|ToString(Integer) (Class|SPlayerState|GetRoundPersonalBest _assplayer_state)) true true "(R=1.000000,G=0.000000,B=0.365323,A=1.000000)")))

(event Input|KeyboardEvents|L
  (params (Key :type Key%20Structure :default "None"))
  ;[1 0 0] DEBUG: TMP Save game
  (:Pressed
    (bind _assgame_mode_base (Utilities|Casting|CastToSGameModeBase (Game|GetGameMode)))
    (Class|SGameModeBase|WriteSaveGame _assgame_mode_base)
    (Development|PrintString "WORLD SAVED")))

(fn ConstructionScript)