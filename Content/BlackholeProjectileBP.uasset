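; Black hole projectile actor that lives briefly, affecting nearby objects with a radial force and swallowing those it overlaps.
; Tick fires the RadialForce impulse every frame and draws a debug sphere around it.
; Sphere overlaps pass through a tag check meant to select Simulating, not-yet-Sucked actors, which then get tagged Sucked.
; The SuckAnim timeline repeatedly multiplies the actor's current scale by its alpha, then destroys it.
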(event OnComponentBeginOverlap(SphereComponent)
  (params (OverlappedComponent :type Primitive%20Component%20Object%20Reference) (OtherActor :type Actor%20Object%20Reference) (OtherComp :type Primitive%20Component%20Object%20Reference) (OtherBodyIndex :type Integer) (bFromSweep :type Boolean) (SweepResult :type Hit%20Result%20Structure%20%28by%20ref%29))
  (if (|HaveCorrectTags? OtherActor)
    (|AddSuckedTag OtherActor)
    (bind _alpha (Timeline|SuckAnim Play)
      (:Update
        (Transformation|SetActorScale3D OtherActor (* _alpha (Transformation|GetActorScale3D OtherActor))))
      (:Finished
        (Actor|DestroyActor OtherActor)))))

(event EventBeginPlay
  (Actor|SetLifeSpan 5.0))

(event Collision|EventActorBeginOverlap
  (params (OtherActor :type Actor%20Object%20Reference)))

(event EventTick
  (params (DeltaSeconds :type Float%20%28single-precision%29))
  (bind _radialforce (Variables|Default|GetRadialForce))
  (Class|RadialForceComponent|FireImpulse _radialforce)
  (Rendering|Debug|DrawDebugSphere (Transformation|GetWorldLocation _radialforce) 6e+02 12 "(R=1.000000,G=0.272174,B=0.382050,A=1.000000)" 0.0))

(fn ConstructionScript)