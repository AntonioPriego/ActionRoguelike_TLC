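; Explosive barrel actor that damages actors it hits and can explode with a radial impulse.
; A static mesh hit applies a fixed health loss to the other actor's SAttributesComponent; this path does not trigger the explosion.
; Explode calls MulticastExplode on server and clients to fire the RadialForceComponent, hide the actor and disable collision.
; A short life span delays destruction so clients receive the multicast first.
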(event OnComponentHit(StaticMeshComponent)
  (params (HitComponent :type Primitive%20Component%20Object%20Reference) (OtherActor :type Actor%20Object%20Reference) (OtherComp :type Primitive%20Component%20Object%20Reference) (NormalImpulse :type Vector :default "0, 0, 0") (Hit :type Hit%20Result%20Structure%20%28by%20ref%29))
  (bind _returnvalue (Actor|GetComponentbyClass OtherActor "/Script/ActionRoguelike_TLC.SAttributesComponent"))
  (Utilities|IsValid OtherActor
    (:Is%20Valid
      (Utilities|IsValid _returnvalue
        (:Is%20Valid
          (Class|SAttributesComponent|ApplyHealthChange _returnvalue 0 -5e+01))))))

(event Custom|Explode
  ;[0.3229 1 0.3287] This way, it will do the stuff in both server and client
  (CallFunction|MulticastExplode)
  (Actor|SetLifeSpan 2.0) ; Wait to destroy the actor to give time to clients to apply the previous node
)

(event Custom|MulticastExplode
  ;[0.3229 1 0.3287] Apply explosion force
  (Class|RadialForceComponent|FireImpulse (Variables|Default|GetRadialForceComponent))
  ;[0.3229 1 0.3287] Set actor non interactable
  (Rendering|SetActorHiddenInGame true)
  (Collision|SetActorEnableCollision false))

(event EventBeginPlay)

(event Collision|EventActorBeginOverlap
  (params (OtherActor :type Actor%20Object%20Reference)))

(event EventTick
  (params (DeltaSeconds :type Float%20%28single-precision%29)))

(fn ConstructionScript)